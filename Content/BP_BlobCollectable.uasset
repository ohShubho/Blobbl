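; Collectable blob pickup that a BP_BlobCharacter collects by overlapping its sphere.
; On overlap, an Attraction timeline lerps the blob mesh toward the character, but its first update also calls CollectedBlob on the character and destroys the pickup.
; The construction script gives each blob a random colour from a fixed palette through the BlobPointColour material parameter.
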(event OnComponentBeginOverlap(Sphere)
  (params (OverlappedComponent :type Primitive%20Component%20Object%20Reference) (OtherActor :type Actor%20Object%20Reference) (OtherComp :type Primitive%20Component%20Object%20Reference) (OtherBodyIndex :type Integer) (bFromSweep :type Boolean) (SweepResult :type Hit%20Result%20Structure%20%28by%20ref%29))
  ;[1 0 0.9043] Once the plater collides with a blob
  (bind _asbp_blob_character (Utilities|Casting|CastToBP_BlobCharacter OtherActor))
  ;[1 0 0.9043] Pull blobs to center of character, just a nice touch
  (bind _distance (Timeline|Attraction Play)
    (:Update
      (Transformation|SetWorldLocation (Variables|Default|GetBlob) (Math|Vector|Lerp(Vector) (Transformation|GetWorldLocation (Variables|Default|GetBlob)) (Transformation|GetActorLocation _asbp_blob_character) _distance) false false)
      ;[1 0 0.9043] Call "Collected Blob" Function then remove blob from game
      (Default|CollectedBlob _asbp_blob_character)
      (Actor|DestroyActor))
    (:Finished
      (Actor|DestroyActor))))

(event EventBeginPlay)

(fn ConstructionScript
  (bind _returnvalue (Math|Conversions|ToVector(LinearColor) "(R=1.000000,G=0.996493,B=0.000000,A=1.000000)"))
  (bind _returnvalue_2 (Math|Conversions|ToVector(LinearColor) "(R=1.000000,G=0.015298,B=0.000000,A=1.000000)"))
  (bind _returnvalue_3 (Math|Conversions|ToVector(LinearColor) "(R=1.000000,G=0.000000,B=0.862875,A=1.000000)"))
  (bind _returnvalue_4 (Math|Conversions|ToVector(LinearColor) "(R=0.000000,G=0.863670,B=1.000000,A=1.000000)"))
  (bind _returnvalue_5 (Math|Conversions|ToVector(LinearColor) "(R=0.000000,G=0.134869,B=1.000000,A=1.000000)"))
  (bind _returnvalue_6 (Math|Conversions|ToVector(LinearColor) "(R=0.000000,G=1.000000,B=0.065165,A=1.000000)"))
  (bind _array (Utilities|Array|MakeArray _returnvalue_2 _returnvalue_3 _returnvalue_4 _returnvalue_5 _returnvalue_6 _returnvalue))
  ;[1 0 0.48] Basically randomizes the colours of the bolbs when the game starts. Will have to incorporate a spawner system to generate blobs throughout game
  (Rendering|Material|SetVectorParameterValueonMaterials (Variables|Default|GetBlob) "BlobPointColour" (Utilities|Array|Get(acopy) _array (Math|Random|RandomIntegerinRange 0 (Utilities|Array|LastIndex _array)))))