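; Player blob character that follows the mouse cursor and grows as it collects blobs.
; Tick sends it toward the cursor hit location with SimpleMoveToLocation.
; CollectedBlob increments and broadcasts the score, lowers walk speed by a flat step once the score reaches five, then enlarges the sphere and lengthens the spring arm to zoom out.
; A debug key triggers the growth and zoom step directly.
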(event Custom|CollectedBlob
  (Utilities|FlowControl|Sequence
    (:then_0
      ;[0 1 0.1571 1 14] Adds score
      (bind _output_get (Variables|Default|SetBlobScore (+ (Variables|Default|GetBlobScore) 1)))
      (Default|CallBlobCollected _output_get))
    (:then_1
      ;[0 1 0.1571 1 14] If score surpasses 5 then start slowing down character. This is most likely going to be removed tho
      (if (>= (Variables|Default|GetBlobScore) 5)
        ;[0 1 0.1571 1 14] Slows player down, updates current speed, prints to screen
        (Variables|/Script/Engine.CharacterMovementComponent|SetMaxWalkSpeed (Variables|Character|GetCharacterMovement) (- (Variables|Default|GetCurrentSpeed) (Variables|Default|GetChangeSpeed)))
        (bind _output_get_2 (Variables|Default|SetCurrentSpeed (- (Variables|Default|GetCurrentSpeed) (Variables|Default|GetChangeSpeed))))
        (Development|PrintString (Utilities|String|ToString(Float) _output_get_2))))
    (:then_2
      ;[1 0.1817 0] Changes size and updates current size
      (Transformation|SetWorldScale3D (Variables|Default|GetSphere) (+ (Variables|Default|Getcurrent%20scale) (Variables|Default|GetAddSize)))
      (Variables|Default|Setcurrent%20scale (Transformation|GetWorldScale (Variables|Default|GetSphere)))
      ;[1 0.1817 0] Changes camera distance, basically zooms out
      (Variables|/Script/Engine.SpringArmComponent|SetTargetArmLength (Variables|Default|GetSpringArm) (+ (Variables|/Script/Engine.SpringArmComponent|GetTargetArmLength (Variables|Default|GetSpringArm)) 3e+02)))))

(event EventTick
  (params (DeltaSeconds :type Float%20%28single-precision%29))
  (bind _returnvalue (Game|GetPlayerController 0))
  ;[0 0.2554 1 1 14] Every the player moves to the mouse location
  (AI|Navigation|SimpleMovetoLocation _returnvalue (.Location (Collision|BreakHitResult (.HitResult (Game|Player|GetHitResultUnderCursorbyChannel _returnvalue "TraceTypeQuery1" true))))))

(event EventBeginPlay
  ;[0 0.2554 1 1 14] Establishes the player's blob starting scale
  (Transformation|SetWorldScale3D (Variables|Default|GetSphere) "4.000000,4.000000,4.000000")
  (Variables|Default|Setcurrent%20scale (Transformation|GetWorldScale (Variables|Default|GetSphere)))
  ;[0 0.2554 1 1 14] Shows mouse cursor
  (Variables|/Script/Engine.PlayerController|SetbShowMouseCursor (Game|GetPlayerController 0) true))

(event Input|KeyboardEvents|1
  (params (Key :type Key%20Structure :default "None"))
  ;[1 1 1] debugging "hotkey"
  (:Pressed
    ;[1 0.1817 0] Changes size and updates current size
    (Transformation|SetWorldScale3D (Variables|Default|GetSphere) (+ (Variables|Default|Getcurrent%20scale) (Variables|Default|GetAddSize)))
    (Variables|Default|Setcurrent%20scale (Transformation|GetWorldScale (Variables|Default|GetSphere)))
    ;[1 0.1817 0] Changes camera distance, basically zooms out
    (Variables|/Script/Engine.SpringArmComponent|SetTargetArmLength (Variables|Default|GetSpringArm) (+ (Variables|/Script/Engine.SpringArmComponent|GetTargetArmLength (Variables|Default|GetSpringArm)) 3e+02))))

(fn ConstructionScript)